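; Recycling bin actor for the trash-in sorting minigame, typed as paper, cans or plastic.
; Touching a bin while time remains sends the assigned trash toward it, then asks the spawner for the next piece or, if none remain, flags every bin to stop accepting input.
; Trash entering the bin's box is destroyed, scoring positive or negative on the main character depending on whether its type matches.
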(event `self.ReceiveBeginPlay`
  (bind _outactors (`GameplayStatics.GetAllActorsOfClass` "/Game/MyAssets/Minigames/trash-in/thrash_spawner_BP.thrash_spawner_BP_C"))
  (set `self.ThrashSpawner_Ref` (`|GetArrayItem` _outactors))
  (bind _astrash_in_main_character (cast `/Game/MyAssets/Minigames/trash-in/trash_in_MainCharacter` (`Controller.K2_GetPawn` (`GameplayStatics.GetPlayerController` 0))))
  (set `self.MainCharacter_ref` _astrash_in_main_character))

(event `self.ReceiveTick`
  (params (DeltaSeconds :type "Float (single-precision)")))

(event `self.StaticMeshComponent.OnInputTouchBegin`
  (params (FingerIndex :type "ETouchIndex Enum" :default "Touch1") (TouchedComponent :type "PrimitiveComponent Object Reference"))
  (bind _trashspawned (`self.trashSpawned`))
  (if (and (not (`self.IsLastTrash`)) (> (`/Game/MyAssets/Minigames/trash-in/trash_in_MainCharacter.timer` (`self.MainCharacter_ref`)) 0.0))
    (`/Engine/EditorBlueprintResources/StandardMacros.IsValid` _trashspawned
      (:`Is Valid`
        (`/Game/MyAssets/Minigames/trash-in/Trash_BP.MoveToBin` _trashspawned (`self.K2_GetActorLocation`))
        (if (== (`/Game/MyAssets/Minigames/trash-in/trash_in_MainCharacter.trashAmountToSpawn` (`self.MainCharacter_ref`)) 0)
          (set `self.IsLastTrash` true)
          (bind _outactors (`GameplayStatics.GetAllActorsOfClass` "Bins_BP_C"))
          (for _array_element _outactors
            (set `/Game/MyAssets/Minigames/trash-in/Bins_BP.IsLastTrash` true _array_element))
          (else
            (`/Game/MyAssets/Minigames/trash-in/thrash_spawner_BP.SpawnNewThrash` (`self.ThrashSpawner_Ref`))))))))

(event `AssignSelectedThrash`
  (params (thash :type "/Game/MyAssets/Minigames/trash-in/Trash_BP Object Reference"))
  (set `self.trashSpawned` thash))

(event `self.Box.OnComponentBeginOverlap`
  (params (OverlappedComponent :type "PrimitiveComponent Object Reference") (OtherActor :type "Actor Object Reference") (OtherComp :type "PrimitiveComponent Object Reference") (OtherBodyIndex :type Integer) (bFromSweep :type Boolean) (SweepResult :type "HitResult Structure (by ref)"))
  (bind _bintype (`self.binType`))
  (bind _astrash_bp (cast `/Game/MyAssets/Minigames/trash-in/Trash_BP` OtherActor))
  (switch `/Game/MyAssets/Minigames/trash-in/TypesofThrash` _bintype
    (:`NewEnumerator0`
      _)
    (:`NewEnumerator1`
      _)
    (:`NewEnumerator2`
      _))
  (if (`|EnumEquality` _bintype (`/Game/MyAssets/Minigames/trash-in/Trash_BP.Thrashtype` _astrash_bp))
    (`/Game/MyAssets/Minigames/trash-in/trash_in_MainCharacter.getPosScore` (`self.MainCharacter_ref`) (`self.binType`))
    (else
      (`/Game/MyAssets/Minigames/trash-in/trash_in_MainCharacter.getNegScore` (`self.MainCharacter_ref`))))
  (cast `/Game/MyAssets/Minigames/trash-in/Trash_BP` OtherActor)
  (`self.K2_DestroyActor` OtherActor))

(fn `UserConstructionScript`)