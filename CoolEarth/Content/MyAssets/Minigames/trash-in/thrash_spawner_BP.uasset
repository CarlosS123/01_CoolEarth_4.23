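; Spawner actor for the trash-in minigame that spawns a random piece of trash and registers it with the bins.
; The construction script caches the actor's location as the spawn point.
; SpawnNewThrash runs on BeginPlay, spawning a random class from the TrashBins array at that point and storing it as SpawnedTrash.
; It then passes the new actor to every Bins_BP in the level through AssignSelectedThrash.
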(event `SpawnNewThrash`
  (bind _trashbins (`self.TrashBins`))
  (bind _returnvalue (`|SpawnActorFromClass` (`|GetArrayItem` _trashbins (`KismetMathLibrary.RandomIntegerInRange` 0 (- (`KismetArrayLibrary.Array_Length` _trashbins) 1))) (`KismetMathLibrary.MakeTransform` (`self.spawnLocation`)) "Undefined" "OverrideRootScale" null null))
  (set `self.SpawnedTrash` _returnvalue)
  (bind _outactors (`GameplayStatics.GetAllActorsOfClass` "/Game/MyAssets/Minigames/trash-in/Bins_BP.Bins_BP_C"))
  (for _array_element _outactors
    (`/Game/MyAssets/Minigames/trash-in/Bins_BP.AssignSelectedThrash` _array_element (`self.SpawnedTrash`))))

(event `self.ReceiveBeginPlay`
  (`self.SpawnNewThrash`))

(fn `UserConstructionScript`
  (set `self.spawnLocation` (`self.K2_GetActorLocation`)))