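; Trash item actor for the trash-in minigame that glides from where it spawned to a tapped bin location.
; On BeginPlay it records its start location and calls DecreaseTrash on the player's trash-in character.
; MoveToBin stores the target and starts movement, which Tick applies as a swept location lerp.
; The alpha's step shrinks as it approaches one, giving an ease-out that slows near the bin.
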(event `self.ReceiveBeginPlay`
  (set `self.startedLocation` (`self.K2_GetActorLocation`))
  (bind _astrash_in_main_character (cast `/Game/MyAssets/Minigames/trash-in/trash_in_MainCharacter` (`GameplayStatics.GetPlayerPawn` 0)))
  (`/Game/MyAssets/Minigames/trash-in/trash_in_MainCharacter.DecreaseTrash` _astrash_in_main_character))

(event `self.ReceiveTick`
  (params (DeltaSeconds :type "Float (single-precision)"))
  (if (`self.isOnTheWay`)
    (set `self.alpha` (`KismetMathLibrary.FClamp` (+ (`self.alpha`) (* DeltaSeconds (`KismetMathLibrary.Lerp` 1.0 0.0 (`self.alpha`))))))
    (`self.K2_SetActorLocation` (`KismetMathLibrary.VLerp` (`self.startedLocation`) (`self.targetBin`) (`self.alpha`)) true)))

(event `MoveToBin`
  (params (binTappedLocation :type "Vector Structure"))
  (set `self.targetBin` binTappedLocation)
  (set `self.isOnTheWay` true))

(fn `UserConstructionScript`)