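; Tetris minigame block actor that dissolves and removes itself when destroyed.
; The Destruction event creates dynamic material instances for the cube, both capsule material slots and the two corn meshes, then sets a destruction flag.
; While flagged, Tick raises a time-based alpha into each material's "Amount" parameter and destroys the actor once it reaches full, about two seconds later.
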(event `self.ReceiveActorBeginOverlap`
  (params (OtherActor :type "Actor Object Reference")))

(event `self.ReceiveTick`
  (params (DeltaSeconds :type "Float (single-precision)"))
  (bind _desintegrationalpha (`self.DesintegrationAlpha`))
  (if (`self.IsBeingDestroyed`)
    (set `self.DesintegrationAlpha` (+ (* DeltaSeconds 0.5) (`self.DesintegrationAlpha`)))
    (`MaterialInstanceDynamic.SetScalarParameterValue` (`self.CubeMaterial`) "Amount" _desintegrationalpha)
    (`MaterialInstanceDynamic.SetScalarParameterValue` (`self.CapsuleMaterial`) "Amount" (`self.DesintegrationAlpha`))
    (`MaterialInstanceDynamic.SetScalarParameterValue` (`self.CornMaterial1`) "Amount" (`self.DesintegrationAlpha`))
    (`MaterialInstanceDynamic.SetScalarParameterValue` (`self.CornMaterial2`) "Amount" (`self.DesintegrationAlpha`))
    (`MaterialInstanceDynamic.SetScalarParameterValue` (`self.CapsuleMaterial2`) "Amount" (`self.DesintegrationAlpha`))
    (if (>= _desintegrationalpha 1.0)
      (`self.K2_DestroyActor`))))

(event `Destruction`
  (bind _capsule (`self.Capsule`))
  (bind _cube (`self.Cube`))
  (bind _capsule_2 (`self.Capsule`))
  (bind _corn1 (`self.Corn1`))
  (bind _corn2 (`self.Corn2`))
  (bind _returnvalue (`PrimitiveComponent.CreateDynamicMaterialInstance` _cube 0 (`PrimitiveComponent.GetMaterial` _cube 0) "None"))
  (set `self.CubeMaterial` _returnvalue)
  (bind _returnvalue_2 (`PrimitiveComponent.CreateDynamicMaterialInstance` _capsule 0 (`PrimitiveComponent.GetMaterial` _capsule 0) "None"))
  (set `self.CapsuleMaterial` _returnvalue_2)
  (bind _returnvalue_3 (`PrimitiveComponent.CreateDynamicMaterialInstance` _capsule_2 1 (`PrimitiveComponent.GetMaterial` _capsule_2 1) "None"))
  (set `self.CapsuleMaterial2` _returnvalue_3)
  (bind _returnvalue_4 (`PrimitiveComponent.CreateDynamicMaterialInstance` _corn1 0 (`PrimitiveComponent.GetMaterial` _corn1 0) "None"))
  (set `self.CornMaterial1` _returnvalue_4)
  (bind _returnvalue_5 (`PrimitiveComponent.CreateDynamicMaterialInstance` _corn2 0 (`PrimitiveComponent.GetMaterial` _corn2 0) "None"))
  (set `self.CornMaterial2` _returnvalue_5)
  (set `self.IsBeingDestroyed` true))

(fn `UserConstructionScript`)