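; Tetris minigame HUD Blueprint that puts the game HUD and pause screen widgets on the viewport.
; BeginPlay creates the TetrisHUD widget for player 0 if no valid instance exists, then displays it.
; The AddPause event does the same for Pause_Screen, reusing the cached widget, with no removal logic here.
; Tick casts the game mode to Tetris_GM but does nothing further.
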(event `self.ReceiveBeginPlay`
  (`/Engine/EditorBlueprintResources/StandardMacros.IsValid` (`self.Tetris_HUD_Widget`)
    (:`Is Valid`
      _)
    (:`Is Not Valid`
      (bind _returnvalue (`|CreateWidget` "/Game/MyAssets/Minigames/TetrisForReal/UI/TetrisHUD.TetrisHUD_C" (`GameplayStatics.GetPlayerController` 0)))
      (set `self.Tetris_HUD_Widget` _returnvalue)))
  (`UserWidget.AddToViewport` (`self.Tetris_HUD_Widget`) 0))

(event `self.ReceiveTick`
  (params (DeltaSeconds :type "Float (single-precision)"))
  (cast `/Game/MyAssets/Minigames/TetrisForReal/Tetris_GM` (`GameplayStatics.GetGameMode`)))

(event `AddPause`
  (`/Engine/EditorBlueprintResources/StandardMacros.IsValid` (`self.PauseWidget`)
    (:`Is Valid`
      _)
    (:`Is Not Valid`
      (bind _returnvalue (`|CreateWidget` "/Game/MyAssets/Minigames/TetrisForReal/UI/Pause_Screen.Pause_Screen_C" (`GameplayStatics.GetPlayerController` 0)))
      (set `self.PauseWidget` _returnvalue)))
  (`UserWidget.AddToViewport` (`self.PauseWidget`) 0))

(fn `UserConstructionScript`)