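; Player controller for the beach minigame that counts down the time remaining in a wave.
; On BeginPlay it casts the game mode to BeachMinigame_GM and copies its WaveTime as the starting value.
; Tick subtracts delta time and prints the remaining time on every frame as debug output, with no clamp or action at zero.
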(event `self.ReceiveBeginPlay`
  (bind _asbeach_minigame_gm (cast `/Game/MyAssets/Blueprints/Beach_MiniGame/BeachMinigame_GM` (`GameplayStatics.GetGameMode`)))
  (set `self.RemainingTime` (`/Game/MyAssets/Blueprints/Beach_MiniGame/BeachMinigame_GM.WaveTime` _asbeach_minigame_gm)))

(event `self.ReceiveTick`
  (params (DeltaSeconds :type "Float (single-precision)"))
  (set `self.DeltaTime` DeltaSeconds)
  (bind _output_get (set `self.RemainingTime` (- (`self.RemainingTime`) (`self.DeltaTime`))))
  (`KismetSystemLibrary.PrintString` (`KismetStringLibrary.Conv_DoubleToString` _output_get) true true (struct :`G` 0.66 :`B` 1.0 :`A` 1.0) 30.0))

(fn `UserConstructionScript`)