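; Player character for an endless runner that runs forward automatically every tick until death, with player-controlled sideways movement and montage-backed jumping.
; When CanTurn is set, left or right input rotates DesiredRotation and the spring arm by ninety degrees, then clears the flag.
; Tick smoothly interpolates control rotation toward that target.
; Death disables input and spawns an explosion effect and sound, while AddCoin increments the coin total.
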(event `self.ReceiveTick`
  (params (DeltaSeconds :type "Float (single-precision)"))
  (if (not (`self.IsDead`))
    (`self.TurnCorner`)
    (`self.AddMovementInput` (`KismetMathLibrary.GetForwardVector` (`KismetMathLibrary.MakeRotator` 0.0 0.0 (.yaw (`self.GetControlRotation`)))))))

(event `InputAction|TurnLeft`
  (params (Key :type "Key Structure"))
  (:`Pressed`
    (if (`self.CanTurn`)
      (set `self.DesiredRotation` (`KismetMathLibrary.ComposeRotators` (`self.DesiredRotation`) (struct :`Yaw` -90.0)))
      (`SceneComponent.K2_SetWorldRotation` (`self.SpringArm1`) (`KismetMathLibrary.ComposeRotators` (`SceneComponent.K2_GetComponentRotation` (`self.SpringArm1`)) (struct :`Yaw` -90.0)) false false)
      (set `self.CanTurn` false :!label _label))))

(event `InputAction|TurnRight`
  (params (Key :type "Key Structure"))
  (:`Pressed`
    (if (`self.CanTurn`)
      (set `self.DesiredRotation` (`KismetMathLibrary.ComposeRotators` (`self.DesiredRotation`) (struct :`Yaw` 90.0)))
      (`SceneComponent.K2_SetWorldRotation` (`self.SpringArm1`) (`KismetMathLibrary.ComposeRotators` (`SceneComponent.K2_GetComponentRotation` (`self.SpringArm1`)) (struct :`Yaw` 90.0)) false false)
      (goto _label))))

(event `InputAction|Jump`
  (params (Key :type "Key Structure"))
  (:`Pressed`
    (`self.Jump`)
    (`self.PlayAnimMontage` "/Game/MyAssets/Characters/RunnerCharacter/Animations/JumpMontage.JumpMontage"))
  (:`Released`
    (`self.StopJumping`)))

(event `InputAxis|MoveRight`
  (params (AxisValue :type "Float (single-precision)"))
  (`self.AddMovementInput` (`KismetMathLibrary.GetRightVector` (`KismetMathLibrary.MakeRotator` 0.0 0.0 (.yaw (`self.GetControlRotation`)))) AxisValue))

(event `TurnCorner`
  (bind _returnvalue (`self.GetControlRotation`))
  (bind _desiredrotation (`self.DesiredRotation`))
  (if (!= _returnvalue _desiredrotation)
    (`Controller.SetControlRotation` (`GameplayStatics.GetPlayerController` 0) (`KismetMathLibrary.RInterpTo` _returnvalue _desiredrotation (`GameplayStatics.GetWorldDeltaSeconds`) 10.0))))

(event `Death`
  (bind _returnvalue (`self.K2_GetActorLocation`))
  (set `self.IsDead` true)
  (`self.DisableInput` null)
  (`GameplayStatics.SpawnEmitterAtLocation` "/Game/MyAssets/Characters/RunnerCharacter/P_EndlessDeath.P_EndlessDeath" _returnvalue)
  (`GameplayStatics.PlaySoundAtLocation` "/Game/MobileStarterContent/Audio/Explosion_Cue.Explosion_Cue" _returnvalue (struct) 1.0 1.0 0.0 null null null))

(fn `AddCoin`
  (set `self.TotalCoins` (+ (`self.TotalCoins`) 1)))

(fn `UserConstructionScript`)