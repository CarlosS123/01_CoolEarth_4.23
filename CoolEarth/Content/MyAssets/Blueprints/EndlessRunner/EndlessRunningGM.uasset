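; Game mode for an endless runner that creates the run HUD and builds the starting track on BeginPlay.
; Ten AddFloorTile calls spawn random straight tiles, each placed at the previous tile's attach transform, stored as NextSpawnPoint.
; A straight counter swaps in a random curve from a separate array once it passes seven, then resets, so turns appear at regular intervals.
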(event `self.ReceiveBeginPlay`
  (bind _returnvalue (`|CreateWidget` "/Game/MyAssets/Blueprints/EndlessRunner/RunHud_WB.RunHud_WB_C"))
  (`UserWidget.AddToViewport` _returnvalue 0)
  (for _ (range 10)
    (`self.AddFloorTile`)))

(fn `AddFloorCurve`
  (bind _floorcurves (`self.FloorCurves`))
  (bind _returnvalue (`|SpawnActorFromClass` (`|GetArrayItem` _floorcurves (`KismetMathLibrary.RandomIntegerInRange` 0 (`KismetArrayLibrary.Array_LastIndex` _floorcurves))) (`self.NextSpawnPoint`) "Undefined" "OverrideRootScale" null null))
  (bind _asfloor_tile_bp (cast `/Game/MyAssets/Blueprints/EndlessRunner/FloorTile_BP` _returnvalue))
  (bind _attachtransform (`/Game/MyAssets/Blueprints/EndlessRunner/FloorTile_BP.GetAttachTransform` _asfloor_tile_bp))
  (set `self.NextSpawnPoint` _attachtransform))

(fn `AddFloorTile`
  (bind _floortiles (`self.FloorTiles`))
  (if (> (`self.CurrentStraights`) 7)
    (`self.AddFloorCurve`)
    (set `self.CurrentStraights` 0)
    (else
      (bind _returnvalue (`|SpawnActorFromClass` (`|GetArrayItem` _floortiles (`KismetMathLibrary.RandomIntegerInRange` 0 (`KismetArrayLibrary.Array_LastIndex` _floortiles))) (`self.NextSpawnPoint`) "Undefined" "OverrideRootScale" null null))
      (bind _asfloor_tile_bp (cast `/Game/MyAssets/Blueprints/EndlessRunner/FloorTile_BP` _returnvalue))
      (bind _attachtransform (`/Game/MyAssets/Blueprints/EndlessRunner/FloorTile_BP.GetAttachTransform` _asfloor_tile_bp))
      (set `self.NextSpawnPoint` _attachtransform)
      (set `self.CurrentStraights` (+ (`self.CurrentStraights`) 1)))))

(fn `UserConstructionScript`)