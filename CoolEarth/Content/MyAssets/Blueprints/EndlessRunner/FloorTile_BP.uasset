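; Floor tile for an endless runner that randomly dresses itself on construction with either five scattered coins or one blocker at one of three spawn points.
; When the runner overlaps the end trigger, it asks the game mode for another tile and destroys itself shortly after.
; Wall hits kill the runner only when head-on, tested by dotting hit normal with forward vector.
; An attach point transform is exposed through a getter.
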(event `self.EndTrigger.OnComponentBeginOverlap`
  (params (OverlappedComponent :type "PrimitiveComponent Object Reference") (OtherActor :type "Actor Object Reference") (OtherComp :type "PrimitiveComponent Object Reference") (OtherBodyIndex :type Integer) (bFromSweep :type Boolean) (SweepResult :type "HitResult Structure (by ref)"))
  (cast `/Game/MyAssets/Blueprints/EndlessRunner/EndlessRunningGuy_BP` OtherActor)
  (bind _asendless_running_gm (cast `/Game/MyAssets/Blueprints/EndlessRunner/EndlessRunningGM` (`GameplayStatics.GetGameMode`)))
  (`/Game/MyAssets/Blueprints/EndlessRunner/EndlessRunningGM.AddFloorTile` _asendless_running_gm)
  (`KismetSystemLibrary.Delay` 0.1)
  (`self.K2_DestroyActor`))

(event `self.Wall.OnComponentHit`
  (params (HitComponent :type "PrimitiveComponent Object Reference") (OtherActor :type "Actor Object Reference") (OtherComp :type "PrimitiveComponent Object Reference") (NormalImpulse :type "Vector Structure") (Hit :type "HitResult Structure (by ref)"))
  (bind _asendless_running_guy_bp (cast `/Game/MyAssets/Blueprints/EndlessRunner/EndlessRunningGuy_BP` OtherActor))
  (if (`KismetMathLibrary.NearlyEqual_FloatFloat` (`KismetMathLibrary.Dot_VectorVector` Hit_Normal (`self.GetActorForwardVector` _asendless_running_guy_bp)) -1.0 0.01)
    (`/Game/MyAssets/Blueprints/EndlessRunner/EndlessRunningGuy_BP.Death` _asendless_running_guy_bp)))

(event `self.Wall2.OnComponentHit`
  (params (HitComponent :type "PrimitiveComponent Object Reference") (OtherActor :type "Actor Object Reference") (OtherComp :type "PrimitiveComponent Object Reference") (NormalImpulse :type "Vector Structure") (Hit :type "HitResult Structure (by ref)"))
  (bind _asendless_running_guy_bp (cast `/Game/MyAssets/Blueprints/EndlessRunner/EndlessRunningGuy_BP` OtherActor))
  (if (`KismetMathLibrary.NearlyEqual_FloatFloat` (`KismetMathLibrary.Dot_VectorVector` Hit_Normal (`self.GetActorForwardVector` _asendless_running_guy_bp)) 1.0 0.01)
    (`/Game/MyAssets/Blueprints/EndlessRunner/EndlessRunningGuy_BP.Death` _asendless_running_guy_bp)))

(fn `GetAttachTransform`
  (returns (AttachTransform :type "Transform Structure"))
  (return (`SceneComponent.K2_GetComponentToWorld` (`self.AttachPoint`))))

(fn `SetSpawnPoints`
  (set `self.SpawnPoints` (`|MakeArray` (`SceneComponent.GetRelativeTransform` (`self.SpawnPointR`)) (`SceneComponent.GetRelativeTransform` (`self.SpawnPointL`)) (`SceneComponent.GetRelativeTransform` (`self.SpawnPoint`)))))

(fn `SpawnBlocker`
  (bind _spawnpoints (`self.SpawnPoints`))
  (`AddComponent|NODE_AddChildActorComponent-0` :`RelativeTransform` (`|GetArrayItem` _spawnpoints (`KismetMathLibrary.RandomIntegerInRange` 0 (`KismetArrayLibrary.Array_LastIndex` _spawnpoints)))))

(fn `SpawnCoins`
  (bind _coinarea (`self.CoinArea`))
  (for _ (range 5)
    (`AddComponent|NODE_AddChildActorComponent-1` :`RelativeTransform` (`KismetMathLibrary.Conv_VectorToTransform` (`KismetMathLibrary.RandomPointInBoundingBox` (`SceneComponent.RelativeLocation` _coinarea) (`BoxComponent.BoxExtent` _coinarea))))))

(fn `UserConstructionScript`
  (`self.SetSpawnPoints`)
  (switch `int` (`KismetMathLibrary.RandomIntegerInRange` 0 1)
    (:`0`
      (`self.SpawnCoins`))
    (:`1`
      (`self.SpawnBlocker`))))