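; MiniGameHUD_BP is a UI manager for a minigame that shows the pause HUD, pause menu, win screen and lose screen.
; On BeginPlay it displays the pause HUD automatically, while separate events show the pause menu, win and lose widgets.
; Each event lazily creates its widget for player 0, caches the reference for reuse, then adds it to the viewport.
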(event `self.ReceiveBeginPlay`
  (`self.Show pause HUD`))

(event `Show pause HUD`
  (`/Engine/EditorBlueprintResources/StandardMacros.IsValid` (`self.PauseWidget_HUD_REF`)
    (:`Is Valid`
      _)
    (:`Is Not Valid`
      (bind _returnvalue (`|CreateWidget` "/Game/MyAssets/Blueprints/UserInterface/PauseHUD_WB.PauseHUD_WB_C" (`GameplayStatics.GetPlayerController` 0)))
      (set `self.PauseWidget_HUD_REF` _returnvalue)))
  (`UserWidget.AddToViewport` (`self.PauseWidget_HUD_REF`) 0))

(event `ShowPauseMenu`
  (`/Engine/EditorBlueprintResources/StandardMacros.IsValid` (`self.Pause_Menu_Widget_REF`)
    (:`Is Valid`
      _)
    (:`Is Not Valid`
      (bind _returnvalue (`|CreateWidget` "/Game/MyAssets/Blueprints/UserInterface/MainPause_WB.MainPause_WB_C" (`GameplayStatics.GetPlayerController` 0)))
      (set `self.Pause_Menu_Widget_REF` _returnvalue)))
  (`UserWidget.AddToViewport` (`self.Pause_Menu_Widget_REF`) 0))

(event `ShowWin`
  (`/Engine/EditorBlueprintResources/StandardMacros.IsValid` (`self.Win_Menu_REF`)
    (:`Is Valid`
      _)
    (:`Is Not Valid`
      (bind _returnvalue (`|CreateWidget` "/Game/MyAssets/Blueprints/UserInterface/MainWin_WB.MainWin_WB_C" (`GameplayStatics.GetPlayerController` 0)))
      (set `self.Win_Menu_REF` _returnvalue)))
  (`UserWidget.AddToViewport` (`self.Win_Menu_REF`) 0))

(event `ShowLose`
  (`/Engine/EditorBlueprintResources/StandardMacros.IsValid` (`self.LoseMenuREF`)
    (:`Is Valid`
      _)
    (:`Is Not Valid`
      (bind _returnvalue (`|CreateWidget` "/Game/MyAssets/Blueprints/UserInterface/MainLose_WB.MainLose_WB_C" (`GameplayStatics.GetPlayerController` 0)))
      (set `self.LoseMenuREF` _returnvalue)))
  (`UserWidget.AddToViewport` (`self.LoseMenuREF`) 0))

(fn `UserConstructionScript`)