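; Grid constructor actor that fills a rectangular area with static mesh components at construction time.
; The construction script steps along X and Y by the separation values up to BoundCorner, adding a component at each grid point.
; Each component gets a random mesh from StaticMeshes using the Seed random stream.
; The event graph has no live logic, only empty events and disconnected GridSpawn and detach nodes.
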(event `self.ReceiveBeginPlay`)

(fn `UserConstructionScript`
  (bind (_boundcorner_x _boundcorner_y) (`KismetMathLibrary.BreakVector` (`self.BoundCorner`)))
  (bind _staticmeshes (`self.StaticMeshes`))
  (bind _staticmeshes_2 (`self.StaticMeshes`))
  (for _index (range (+ (`KismetMathLibrary.FTrunc` (/ _boundcorner_x (`self.XSeparation`))) 1))
    (bind _returnvalue (* _index (`self.XSeparation`)))
    (bind _returnvalue_2 (`AddComponent|NODE_AddStaticMeshComponent-0` :`RelativeTransform` (`KismetMathLibrary.MakeTransform` (`KismetMathLibrary.MakeVector` _returnvalue))))
    (`StaticMeshComponent.SetStaticMesh` _returnvalue_2 (`|GetArrayItem` _staticmeshes_2 (`KismetMathLibrary.RandomIntegerInRangeFromStream` 0 (- (`KismetArrayLibrary.Array_Length` _staticmeshes_2) 1) (`self.Seed`))))
    (for _index_2 (range 1 (+ (`KismetMathLibrary.FTrunc` (/ _boundcorner_y (`self.YSeparation`))) 1))
      (bind _returnvalue_3 (`AddComponent|NODE_AddStaticMeshComponent-1` :`RelativeTransform` (`KismetMathLibrary.MakeTransform` (`KismetMathLibrary.MakeVector` _returnvalue (* _index_2 (`self.YSeparation`))))))
      (`StaticMeshComponent.SetStaticMesh` _returnvalue_3 (`|GetArrayItem` _staticmeshes (`KismetMathLibrary.RandomIntegerInRangeFromStream` 0 (- (`KismetArrayLibrary.Array_Length` _staticmeshes) 1) (`self.Seed`)))))))