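; CrowdCharacter_BP spawns the audience crowd for the speech game when play begins.
; A single loop places 50 characters in five rows of ten, with random spacing and jitter, resetting position and yaw at each new row.
; Yaw increases steadily along each row.
; Each spawn randomly picks businessman, blue collar or hippie and increments that type's counter.
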(event `self.ReceiveBeginPlay`
  (bind (_nextlocation_x _nextlocation_y) (`KismetMathLibrary.BreakVector` (`self.NextLocation`)))
  (for _index (range 50)
    (if (or (== _index 9) (== _index 19) (== _index 29) (== _index 39))
      (set `self.NextLocation` (+ (`KismetMathLibrary.MakeVector` 0.0 _nextlocation_y 890.0) (200.0 -200.0 0.0)))
      (set `self.NextXRotation` -46.0)
      (else
        (set `self.NextLocation` (+ (`self.NextLocation`) (`KismetMathLibrary.MakeVector` (`KismetMathLibrary.RandomFloatInRange` 100.0 180.0) (`KismetMathLibrary.RandomFloatInRange` -25.0 25.0))))
        (set `self.NextXRotation` (- (`self.NextXRotation`) -8.0))))
    (switch `int` (`KismetMathLibrary.RandomInteger` 3)
      (:`0`
        (`|SpawnActorFromClass` "/Game/MyAssets/Blueprints/SpeechGameBP/CrowdBusinessman_BP.CrowdBusinessman_BP_C" (`KismetMathLibrary.MakeTransform` (`self.NextLocation`) (`KismetMathLibrary.MakeRotator` 0.0 0.0 (`self.NextXRotation`))) "Undefined" "OverrideRootScale" null null)
        (set `self.BusinessmanAmount` (+ (`self.BusinessmanAmount`) 1)))
      (:`1`
        (`|SpawnActorFromClass` "/Game/MyAssets/Blueprints/SpeechGameBP/CrowdBlueCollar_BP.CrowdBlueCollar_BP_C" (`KismetMathLibrary.MakeTransform` (`self.NextLocation`) (`KismetMathLibrary.MakeRotator` 0.0 0.0 (`self.NextXRotation`))) "Undefined" "OverrideRootScale" null null)
        (set `self.BlueCollarAmount` (+ (`self.BlueCollarAmount`) 1)))
      (:`2`
        (`|SpawnActorFromClass` "/Game/MyAssets/Blueprints/SpeechGameBP/CrowdHippie_BP.CrowdHippie_BP_C" (`KismetMathLibrary.MakeTransform` (`self.NextLocation`) (`KismetMathLibrary.MakeRotator` 0.0 0.0 (`self.NextXRotation`))) "Undefined" "OverrideRootScale" null null)
        (set `self.HippieAmount` (+ (`self.HippieAmount`) 1))))))

(fn `UserConstructionScript`)