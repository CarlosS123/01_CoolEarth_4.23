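; Player character for the speech game that creates the SpeechGame widget on begin play, shows the mouse cursor and stages a camera move for slides.
; ShowSlide repositions and lengthens the spring arm, then a timeline adds a lerped rotation to it every update.
; EndSlide restores the saved transform but leaves arm length and timeline untouched.
; An IsRotating-based spin is left unwired.
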(event `self.ReceiveBeginPlay`
  (bind _returnvalue (`|CreateWidget` "/Game/MyAssets/Blueprints/SpeechGameBP/SpeechGame_WB.SpeechGame_WB_C"))
  (bind _output_get (set `self.SpeechGameWidget` _returnvalue))
  (`UserWidget.AddToViewport` _returnvalue 0)
  (`UserWidget.AddToViewport` _output_get 0)
  (set `PlayerController.bShowMouseCursor` true (`GameplayStatics.GetPlayerController` 0))
  (set `self.CameraOriginalTransform` (`SceneComponent.GetRelativeTransform` (`self.SpringArm`))))

(event `ShowSlide`
  (set `SpringArmComponent.TargetArmLength` 1000.0 (`self.SpringArm`))
  (`SceneComponent.K2_SetRelativeTransform` (`self.SpringArm`) (`KismetMathLibrary.MakeTransform` (-36.0 0.0 54.0) (struct :`Pitch` -30.0 :`Yaw` -140.0)) false false)
  (bind (_direction _rotation_alpha) (`Timeline|Timeline_0` :!via `PlayFromStart`)
    (:`Update`
      (`SceneComponent.K2_AddRelativeRotation` (`self.SpringArm`) (`KismetMathLibrary.RLerp` (struct :`Pitch` -30.0 :`Yaw` -140.0) (struct :`Pitch` -30.0 :`Yaw` -220.0) _rotation_alpha) false false))))

(event `EndSlide`
  (set `self.IsRotating` false)
  (`SceneComponent.K2_SetRelativeTransform` (`self.SpringArm`) (`self.CameraOriginalTransform`) false false))

(event `self.ReceiveTick`
  (params (DeltaSeconds :type "Float (single-precision)")))

(event `Do rotation`)

(fn `UserConstructionScript`)