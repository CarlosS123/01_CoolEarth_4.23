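; Player controller for a Tetris-style game that turns input actions into moves on the Tetris_GM game mode.
; TurnRight, TurnLeft, Jump and Rotate presses each cast the game mode and call MoveRight, MoveLeft, Down and Rotate respectively.
; Every move is ignored while the game mode's IsDrillBeingRotated flag is set.
; The controller holds no game logic beyond that check.
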(event `InputAction|TurnRight`
  (params (Key :type "Key Structure"))
  (:`Pressed`
    (bind _astetris_gm (cast `/Game/MyAssets/Blueprints/TetrisBP/Tetris_GM` (`GameplayStatics.GetGameMode`)))
    (if (not (`/Game/MyAssets/Blueprints/TetrisBP/Tetris_GM.IsDrillBeingRotated` _astetris_gm))
      (`/Game/MyAssets/Blueprints/TetrisBP/Tetris_GM.MoveRight` _astetris_gm))))

(event `InputAction|TurnLeft`
  (params (Key :type "Key Structure"))
  (:`Pressed`
    (bind _astetris_gm (cast `/Game/MyAssets/Blueprints/TetrisBP/Tetris_GM` (`GameplayStatics.GetGameMode`)))
    (if (not (`/Game/MyAssets/Blueprints/TetrisBP/Tetris_GM.IsDrillBeingRotated` _astetris_gm))
      (`/Game/MyAssets/Blueprints/TetrisBP/Tetris_GM.MoveLeft` _astetris_gm))))

(event `InputAction|Jump`
  (params (Key :type "Key Structure"))
  (:`Pressed`
    (bind _astetris_gm (cast `/Game/MyAssets/Blueprints/TetrisBP/Tetris_GM` (`GameplayStatics.GetGameMode`)))
    (if (not (`/Game/MyAssets/Blueprints/TetrisBP/Tetris_GM.IsDrillBeingRotated` _astetris_gm))
      (`/Game/MyAssets/Blueprints/TetrisBP/Tetris_GM.Down` _astetris_gm))))

(event `InputAction|Rotate`
  (params (Key :type "Key Structure"))
  (:`Pressed`
    (bind _astetris_gm (cast `/Game/MyAssets/Blueprints/TetrisBP/Tetris_GM` (`GameplayStatics.GetGameMode`)))
    (if (not (`/Game/MyAssets/Blueprints/TetrisBP/Tetris_GM.IsDrillBeingRotated` _astetris_gm))
      (`/Game/MyAssets/Blueprints/TetrisBP/Tetris_GM.Rotate` _astetris_gm))))

(fn `UserConstructionScript`)