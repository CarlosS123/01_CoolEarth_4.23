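; Player character for a trash-sorting game that keeps the score counters for binned and wasted trash.
; Scoring events lower the remaining trash count and add a point for paper, cans or plastic, or a negative point.
; A separate event decrements the amount left to spawn.
; BeginPlay and Tick are empty; count setup, HUD timer read, lose message and debug score printouts are disconnected and never run.
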(event `self.ReceiveBeginPlay`)

(event `self.ReceiveTick`
  (params (DeltaSeconds :type "Float (single-precision)")))

(event `getPosScore`
  (params (typeOfBin :type "/Game/MyAssets/Blueprints/Trash-in/TypesofThrash Enum" :default "NewEnumerator0"))
  (`/Engine/EditorBlueprintResources/StandardMacros.DecrementInt` (`self.trashAmountRemaining`)
    (:`  `
      (switch `/Game/MyAssets/Blueprints/Trash-in/TypesofThrash` typeOfBin
        (:`NewEnumerator0`
          (`/Engine/EditorBlueprintResources/StandardMacros.IncrementInt` (`self.pos_points_paper`)))
        (:`NewEnumerator1`
          (`/Engine/EditorBlueprintResources/StandardMacros.IncrementInt` (`self.pos_points_cans`)))
        (:`NewEnumerator2`
          (`/Engine/EditorBlueprintResources/StandardMacros.IncrementInt` (`self.pos_points_plastic`)))))))

(event `getNegScore`
  (`/Engine/EditorBlueprintResources/StandardMacros.DecrementInt` (`self.trashAmountRemaining`)
    (:`  `
      (`/Engine/EditorBlueprintResources/StandardMacros.IncrementInt` (`self.neg_points`)))))

(event `DecreaseTrash`
  (`/Engine/EditorBlueprintResources/StandardMacros.DecrementInt` (`self.trashAmountToSpawn`)))

(fn `UserConstructionScript`)