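; Recycling bin actor for a timed trash-sorting game, labeled with its trash type and an animated arrow.
; A click or touch on its mesh while time remains sends the assigned trash to the bin and has the spawner create another.
; On box overlap it compares trash and bin types, adjusts the main character's score, HUD score and its displayed count, then destroys the trash.
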(event `self.ReceiveBeginPlay`
  (bind _astrash_in_hud_bp (cast `/Game/MyAssets/Blueprints/Trash-in/trash_in_HUD_BP` (`PlayerController.GetHUD` (`GameplayStatics.GetPlayerController` 0))))
  (set `self.HUD_REF` _astrash_in_hud_bp)
  (`TextRenderComponent.K2_SetText` (`self.TypeOfTrash_Text`) (`self.TypeOfTrash`))
  (bind _outactors (`GameplayStatics.GetAllActorsOfClass` "/Game/MyAssets/Blueprints/Trash-in/thrash_spawner_BP.thrash_spawner_BP_C"))
  (set `self.ThrashSpawner_Ref` (`|GetArrayItem` _outactors))
  (bind _astrash_in_main_character (cast `/Game/MyAssets/Blueprints/Trash-in/trash_in_MainCharacter` (`Controller.K2_GetPawn` (`GameplayStatics.GetPlayerController` 0))))
  (set `self.MainCharacter_ref` _astrash_in_main_character)
  (bind (_direction _alpha_transform) (`Timeline|ArrowAnim`)
    (:`Update`
      (`SceneComponent.K2_SetRelativeTransform` (`self.Arrow`) (`KismetMathLibrary.TLerp` (`KismetMathLibrary.MakeTransform` (0.0 0.0 55.0) (struct) (2.0 4.0 2.0)) (`KismetMathLibrary.MakeTransform` (0.0 0.0 45.0) (struct) (1.0 1.0 1.0)) _alpha_transform) false false))))

(event `self.Box.OnClicked`
  (params (TouchedComponent :type "PrimitiveComponent Object Reference") (ButtonPressed :type "Key Structure")))

(event `self.ReceiveTick`
  (params (DeltaSeconds :type "Float (single-precision)")))

(event `self.StaticMeshComponent.OnClicked`
  (params (TouchedComponent :type "PrimitiveComponent Object Reference") (ButtonPressed :type "Key Structure"))
  (bind _trashspawned (`self.trashSpawned`))
  (if (and (not (`self.IsLastTrash`)) (> (`/Game/MyAssets/Blueprints/Trash-in/trash_in_HUD_BP.GameTimeRemainig` (`self.HUD_REF`)) 0.0)) :!label _label
    (`/Engine/EditorBlueprintResources/StandardMacros.IsValid` _trashspawned
      (:`Is Valid`
        (`/Game/MyAssets/Blueprints/Trash-in/Trash_BP.MoveToBin` _trashspawned (`self.K2_GetActorLocation`))
        (`/Game/MyAssets/Blueprints/Trash-in/thrash_spawner_BP.SpawnNewThrash` (`self.ThrashSpawner_Ref`))))))

(event `self.StaticMeshComponent.OnInputTouchBegin`
  (params (FingerIndex :type "ETouchIndex Enum" :default "Touch1") (TouchedComponent :type "PrimitiveComponent Object Reference"))
  (goto _label))

(event `AssignSelectedThrash`
  (params (thash :type "/Game/MyAssets/Blueprints/Trash-in/Trash_BP Object Reference"))
  (set `self.trashSpawned` thash))

(event `self.Box.OnComponentBeginOverlap`
  (params (OverlappedComponent :type "PrimitiveComponent Object Reference") (OtherActor :type "Actor Object Reference") (OtherComp :type "PrimitiveComponent Object Reference") (OtherBodyIndex :type Integer) (bFromSweep :type Boolean) (SweepResult :type "HitResult Structure (by ref)"))
  (bind _bintype (`self.binType`))
  (bind _amount_of_trash_classified (`self.Amount of Trash classified`))
  (bind _astrash_bp (cast `/Game/MyAssets/Blueprints/Trash-in/Trash_BP` OtherActor))
  (switch `/Game/MyAssets/Blueprints/Trash-in/TypesofThrash` _bintype
    (:`NewEnumerator0`
      _)
    (:`NewEnumerator1`
      _)
    (:`NewEnumerator2`
      _))
  (if (`|EnumEquality` _bintype (`/Game/MyAssets/Blueprints/Trash-in/Trash_BP.Thrashtype` _astrash_bp))
    (`/Game/MyAssets/Blueprints/Trash-in/trash_in_MainCharacter.getPosScore` (`self.MainCharacter_ref`) (`self.binType`))
    (`/Engine/EditorBlueprintResources/StandardMacros.IncrementInt` _amount_of_trash_classified
      (:`  `
        (`self.Increase_HUD_score`)))
    (else
      (`/Game/MyAssets/Blueprints/Trash-in/trash_in_MainCharacter.getNegScore` (`self.MainCharacter_ref`))
      (`/Engine/EditorBlueprintResources/StandardMacros.DecrementInt` _amount_of_trash_classified
        (:`  `
          (`self.Decrease_HUD_score`)))))
  (`TextRenderComponent.K2_SetText` (`self.Trash`) (`KismetTextLibrary.Conv_IntToText` _amount_of_trash_classified))
  (`self.K2_DestroyActor` OtherActor))

(event `SetIsGameOver`
  (set `self.IsGameOver` true))

(fn `Decrease_HUD_score`
  (bind _astrash_in_hud_bp (cast `/Game/MyAssets/Blueprints/Trash-in/trash_in_HUD_BP` (`PlayerController.GetHUD` (`GameplayStatics.GetPlayerController` 0))))
  (`/Game/MyAssets/Blueprints/Trash-in/trash_in_HUD_BP.DecreaseScore` _astrash_in_hud_bp))

(fn `Increase_HUD_score`
  (bind _astrash_in_hud_bp (cast `/Game/MyAssets/Blueprints/Trash-in/trash_in_HUD_BP` (`PlayerController.GetHUD` (`GameplayStatics.GetPlayerController` 0))))
  (`/Game/MyAssets/Blueprints/Trash-in/trash_in_HUD_BP.IncreaseScore` _astrash_in_hud_bp))

(fn `UserConstructionScript`
  (bind _textmaterial (`self.TextMaterial`))
  (`PrimitiveComponent.SetMaterial` (`self.TypeOfTrash_Text`) 0 _textmaterial)
  (`PrimitiveComponent.SetMaterial` (`self.Trash`) 0 _textmaterial))