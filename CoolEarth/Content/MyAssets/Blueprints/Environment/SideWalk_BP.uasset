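; SideWalk_BP is an environment Blueprint that builds a straight sidewalk from the actor toward its Endpoint offset.
; The Construction Script turns the base sidewalk mesh to face Endpoint in yaw only, flipped 180 degrees, skipping offsets with no horizontal component.
; It then attaches added mesh components along the base's negative X at ObjLenght spacing, with the count floored from Endpoint's length.
; The Event Graph is unused.
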(fn `UserConstructionScript`
  (bind _returnvalue (`self.K2_GetActorLocation`))
  (bind _objlenght (`self.ObjLenght`))
  (if (!= (* (`self.endpoint`) (1.0 1.0 0.0)) (0.0 0.0 0.0))
    (`SceneComponent.K2_SetWorldRotation` (`self.SM_Env_Sidewalk`) (`KismetMathLibrary.MakeRotator` 0.0 0.0 (+ (.yaw (`KismetMathLibrary.FindLookAtRotation` _returnvalue (+ _returnvalue (`self.endpoint`)))) 180.0)) false false)
    (for _index (range 1 (`KismetMathLibrary.FFloor` (/ (`KismetMathLibrary.VSize` (`self.endpoint`)) _objlenght)))
      (bind _returnvalue_2 (`AddComponent|NODE_AddStaticMeshComponent-5`))
      (`SceneComponent.K2_AttachToComponent` _returnvalue_2 (`self.SM_Env_Sidewalk`) "None" "KeepWorld" "KeepRelative" "KeepWorld" true)
      (`SceneComponent.K2_SetRelativeLocation` _returnvalue_2 (`KismetMathLibrary.MakeVector` (* (* _index _objlenght) -1.0)) false false))))