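; Procedural street actor that builds a straight row of static mesh segments toward an Endpoint offset in the Construction Script.
; When Endpoint's horizontal offset is nonzero, it adds meshes under Street2 along local Y, then yaws Street2 to face that offset.
; Segment count comes from 1000-unit steps of Endpoint's length but spacing is 2200 units, so the row can extend well past Endpoint.
; The Event Graph is unused.
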(fn `UserConstructionScript`
  (bind _returnvalue (`self.K2_GetActorLocation`))
  (if (!= (* (`self.endpoint`) (1.0 1.0 0.0)) (0.0 0.0 0.0))
    (for _index (range (+ (`KismetMathLibrary.FFloor` (/ (`KismetMathLibrary.VSize` (`self.endpoint`)) 1000.0)) 1))
      (bind _returnvalue_2 (`AddComponent|NODE_AddStaticMeshComponent-5` :`RelativeTransform` (`KismetMathLibrary.MakeTransform` (0.0 0.0 0.0) (struct) (1.0 1.0 1.0))))
      (`SceneComponent.K2_AttachToComponent` _returnvalue_2 (`self.street2`) "None" "KeepWorld" "KeepRelative" "KeepWorld" true)
      (`SceneComponent.K2_SetRelativeLocation` _returnvalue_2 (`KismetMathLibrary.MakeVector` 0.0 (* _index 2200.0)) false false))
    (`SceneComponent.K2_SetWorldRotation` (`self.street2`) (`KismetMathLibrary.MakeRotator` 0.0 0.0 (+ (.yaw (`KismetMathLibrary.FindLookAtRotation` _returnvalue (+ _returnvalue (`self.endpoint`)))) -90.0)) false false)))