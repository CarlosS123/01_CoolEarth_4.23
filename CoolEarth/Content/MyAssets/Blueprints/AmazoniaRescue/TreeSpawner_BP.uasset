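; TreeSpawner_BP is a scatter actor that fills an area with randomly chosen tree meshes.
; Its Construction Script loops over TreeCount, picks from TreeArray and adds a static mesh component with random position and height scale.
; The plains stump mesh gets a narrower footprint scale and mostly hardcoded position ranges, while other meshes use the Min/Max X and Y bounds.
; The event graph is empty, so nothing runs during play.
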(event `self.ReceiveBeginPlay`)

(event `self.ReceiveActorBeginOverlap`
  (params (OtherActor :type "Actor Object Reference")))

(event `self.ReceiveTick`
  (params (DeltaSeconds :type "Float (single-precision)")))

(fn `UserConstructionScript`
  (bind _treearray (`self.TreeArray`))
  (for _ (range (+ (`self.TreeCount`) 1))
    (bind _output_get (set `self.SelectedTree` (`|GetArrayItem` _treearray (`KismetMathLibrary.RandomInteger` (`KismetArrayLibrary.Array_Length` _treearray)))))
    (if (== "/Game/MyAssets/StaticMesh/Plains_Tree_Stump01_SM.Plains_Tree_Stump01_SM" _output_get)
      (bind _returnvalue (`AddComponent|NODE_AddStaticMeshComponent-2` :`RelativeTransform` (`KismetMathLibrary.MakeTransform` (`KismetMathLibrary.MakeVector` (`KismetMathLibrary.RandomFloatInRange` -250.0 250.0) (`KismetMathLibrary.RandomFloatInRange` (`self.Max_X`) 250.0) 10.0) (struct) (`KismetMathLibrary.MakeVector` 0.15 0.15 (`KismetMathLibrary.RandomFloatInRange` 0.25 0.35)))))
      (`StaticMeshComponent.SetStaticMesh` _returnvalue (`self.SelectedTree`))
      (else
        (bind _returnvalue_2 (`AddComponent|NODE_AddStaticMeshComponent-0` :`RelativeTransform` (`KismetMathLibrary.MakeTransform` (`KismetMathLibrary.MakeVector` (`KismetMathLibrary.RandomFloatInRange` (`self.Min_X`) (`self.Max_X`)) (`KismetMathLibrary.RandomFloatInRange` (`self.Min_Y`) (`self.Max_Y`)) 10.0) (struct) (`KismetMathLibrary.MakeVector` 0.3 0.3 (`KismetMathLibrary.RandomFloatInRange` 0.25 0.35)))))
        (`StaticMeshComponent.SetStaticMesh` _returnvalue_2 (`self.SelectedTree`))))))