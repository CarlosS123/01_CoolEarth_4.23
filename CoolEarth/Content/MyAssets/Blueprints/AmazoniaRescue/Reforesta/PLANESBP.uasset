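; PLANESBP is a touchable plane actor in the Amazonia Rescue reforestation game, apparently the base for player and enemy planes.
; Until LevelComplete sets its finished flag, a touch checks the plane's type and prints its transform for debugging.
; A Deforestation plane spawns a PLANESBP_Player at the same transform, then destroys itself if it is a PLANESBP_Enemy, turning deforested tiles into player ones.
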(event `self.ReceiveTick`
  (params (DeltaSeconds :type "Float (single-precision)")))

(event `self.Plane.OnInputTouchBegin`
  (params (FingerIndex :type "ETouchIndex Enum" :default "Touch1") (TouchedComponent :type "PrimitiveComponent Object Reference"))
  (bind _returnvalue (`ActorComponent.GetOwner` TouchedComponent))
  (bind _returnvalue_2 (`self.GetTransform` _returnvalue))
  (if (not (`self.LevelFinished`))
    (bind _output_get (set `self.TouchedPlane` _returnvalue))
    (bind _asplanesbp (cast `/Game/MyAssets/Blueprints/AmazoniaRescue/Reforesta/PLANESBP` _output_get))
    (`KismetSystemLibrary.PrintString` (`KismetStringLibrary.Conv_TransformToString` _returnvalue_2))
    (switch `/Game/MyAssets/Minigames/MiniGameAndres/Reforesta/PlaneType` (`/Game/MyAssets/Blueprints/AmazoniaRescue/Reforesta/PLANESBP.PlaneType` _asplanesbp)
      (:`NewEnumerator1`
        (bind _returnvalue_3 (`|SpawnActorFromClass` "/Game/MyAssets/Minigames/MiniGameAndres/Reforesta/PLANESBP_Player.PLANESBP_Player_C" _returnvalue_2 "Undefined" "OverrideRootScale" null false null))
        (bind _asplanesbp_enemy (cast `/Game/MyAssets/Minigames/MiniGameAndres/Reforesta/PLANESBP_Enemy` (`self.TouchedPlane`)))
        (`self.K2_DestroyActor` _asplanesbp_enemy)))))

(event `LevelComplete`
  (params (complete :type Boolean))
  (set `self.LevelFinished` complete))

(fn `UserConstructionScript`)