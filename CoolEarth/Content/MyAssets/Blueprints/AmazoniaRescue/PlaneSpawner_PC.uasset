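; Player controller for the Amazonia Rescue level that tracks score and countdown, and decides when the level ends.
; On BeginPlay it sets Game and UI input, counts all planes and reads the time limit from the game mode.
; Each Tick it recomputes score as the percentage of that initial count that are player planes.
; At full score or time out, it flags itself, every plane and the enemy spawner as level complete.
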(event `self.ReceiveBeginPlay`
  (`WidgetBlueprintLibrary.SetInputMode_GameAndUIEx` (`GameplayStatics.GetPlayerController` 0) null)
  (bind _outactors (`GameplayStatics.GetAllActorsOfClass` "/Game/MyAssets/Blueprints/AmazoniaRescue/PLANES_BP.PLANES_BP_C"))
  (set `self.TotalPlanes` (`KismetArrayLibrary.Array_Length` _outactors))
  (bind _asamazonia_rescue_gm (cast `/Game/MyAssets/Blueprints/AmazoniaRescue/AmazoniaRescue_GM` (`GameplayStatics.GetGameMode`)))
  (set `self.RemainingTime` (`/Game/MyAssets/Blueprints/AmazoniaRescue/AmazoniaRescue_GM.GlobalTime` _asamazonia_rescue_gm)))

(event `self.ReceiveTick`
  (params (DeltaSeconds :type "Float (single-precision)"))
  (set `self.DeltaTime` DeltaSeconds)
  (if (`self.LevelFinished`)
    _
    (elif (> (`self.RemainingTime`) 0.0)
      (bind _outactors (`GameplayStatics.GetAllActorsOfClass` "/Game/MyAssets/Blueprints/AmazoniaRescue/PLANES_BP.PLANES_BP_C"))
      (for _array_element _outactors
        (cast `/Game/MyAssets/Blueprints/AmazoniaRescue/PLANES_Ch_Player_BP` _array_element)
        (`/Engine/EditorBlueprintResources/StandardMacros.IncrementInt` (`self.PlayerPlanes`)))
      (bind _output_get (set `self.Score ` (* (/ (`KismetMathLibrary.Conv_IntToDouble` (`self.PlayerPlanes`)) (`KismetMathLibrary.Conv_IntToDouble` (`self.TotalPlanes`))) 100.0)))
      (set `self.PlayerPlanes` 0)
      (bind _output_get_2 (set `self.StillIncomplete` (< _output_get 100.0)))
      (if _output_get_2
        (set `self.RemainingTime` (- (`self.RemainingTime`) (`self.DeltaTime`)))
        (else
          (bind _outactors_2 (`GameplayStatics.GetAllActorsOfClass` "/Game/MyAssets/Blueprints/AmazoniaRescue/PLANES_BP.PLANES_BP_C"))
          (for _array_element_2 _outactors_2
            (`/Game/MyAssets/Blueprints/AmazoniaRescue/PLANES_BP.LevelComplete ` _array_element_2 true))
          (bind _asenemy_spawner_bp (cast `/Game/MyAssets/Blueprints/AmazoniaRescue/EnemySpawner_BP` (`self.K2_GetPawn`)))
          (`/Game/MyAssets/Blueprints/AmazoniaRescue/EnemySpawner_BP.LevelComplete ` _asenemy_spawner_bp true)
          (`self.LevelComplete ` true)))
      (else
        (`self.LevelComplete ` true)
        (bind _returnvalue (`GameplayStatics.GetActorOfClass` "/Game/MyAssets/Blueprints/AmazoniaRescue/EnemySpawner_BP.EnemySpawner_BP_C"))
        (`/Game/MyAssets/Blueprints/AmazoniaRescue/EnemySpawner_BP.LevelComplete ` _returnvalue true)
        (bind _outactors_3 (`GameplayStatics.GetAllActorsOfClass` "/Game/MyAssets/Blueprints/AmazoniaRescue/PLANES_BP.PLANES_BP_C"))
        (for _array_element_3 _outactors_3
          (`/Game/MyAssets/Blueprints/AmazoniaRescue/PLANES_BP.LevelComplete ` _array_element_3 true))))))

(event `LevelComplete`
  (params (complete :type Boolean))
  (set `self.LevelFinished` complete))

(fn `UserConstructionScript`)