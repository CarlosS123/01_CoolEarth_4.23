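; Enemy Blueprint in AmazoniaRescue, apparently for planes, that extends a parent class and adds setup on spawn.
; On BeginPlay it runs the parent logic, then gives its Scene component a random relative yaw across a full turn.
; When AmITheFirst is true, it also clears the template of ParticleSystem1.
; Overlap and Tick events are disabled stubs, and the construction script only calls the parent.
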(event `self.ReceiveBeginPlay`
  (`parent.ReceiveBeginPlay`)
  (`SceneComponent.K2_SetRelativeRotation` (`self.Scene`) (`KismetMathLibrary.MakeRotator` 0.0 0.0 (`KismetMathLibrary.RandomFloatInRange` 0.0 360.0)) false true)
  (if (`self.AmITheFirst`)
    (`ParticleSystemComponent.SetTemplate` (`self.ParticleSystem1`) null)))

(fn `UserConstructionScript`
  (`parent.UserConstructionScript`))