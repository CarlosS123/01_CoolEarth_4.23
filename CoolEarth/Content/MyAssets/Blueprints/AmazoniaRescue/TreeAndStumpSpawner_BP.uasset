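; TreeAndStumpSpawner_BP is an Amazonia Rescue Blueprint named as a tree and stump spawner, though it only builds a list of stump meshes so far.
; The construction script loops from 0 through StumpCount inclusive, adding the same Plains stump mesh to TreeArray on each pass, one more than the count.
; Nothing here spawns or places those meshes, and the event graph holds only disabled default events.
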(fn `UserConstructionScript`
  (for _ (range (+ (`self.StumpCount`) 1))
    (`KismetArrayLibrary.Array_Add` (`self.TreeArray`) "/Game/MyAssets/StaticMesh/Plains_Tree_Stump01_SM.Plains_Tree_Stump01_SM"))
  (`parent.UserConstructionScript`))