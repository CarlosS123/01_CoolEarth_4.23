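; Tree-cluster actor for Amazonia Rescue whose three trees grow from sprout through growing to mature.
; A placement macro randomly offsets the trees at construction and BeginPlay, storing the owning actor's location for each.
; Until LevelFinished, Tick reapplies the current stage's mesh and scale and calls StateChange, whose Delay advances the stage every ten seconds.
; An AmITheFirst flag resets the particle system template at BeginPlay.
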(event `self.ReceiveBeginPlay`
  (`parent.ReceiveBeginPlay`)
  (`self.Tree_location`)
  (if (`self.AmITheFirst`)
    (`ParticleSystemComponent.SetTemplate` (`self.ParticleSystem`) null)))

(event `self.ReceiveTick`
  (params (DeltaSeconds :type "Float (single-precision)"))
  (`parent.ReceiveTick` DeltaSeconds)
  (if (not (`self.LevelFinished`))
    (switch `/Game/MyAssets/Blueprints/AmazoniaRescue/TreeState_Enum` (`self.TreeState`)
      (:`NewEnumerator0`
        (`self.Sprout`))
      (:`NewEnumerator1`
        (`self.Growth`))
      (:`NewEnumerator2`
        (`self.Mature`)))
    (`self.StateChange` (`self.TreeState`))))

(event `StateChange`
  (params (NewParam :type "/Game/MyAssets/Blueprints/AmazoniaRescue/TreeState_Enum Enum" :default "NewEnumerator0"))
  (`KismetSystemLibrary.Delay` 10.0)
  (if (`|EnumEquality` NewParam "NewEnumerator0")
    (set `self.TreeState` "NewEnumerator1")
    (elif (`|EnumEquality` NewParam "NewEnumerator1")
      (set `self.TreeState` "NewEnumerator2"))))

(fn `UserConstructionScript`
  (`parent.UserConstructionScript`)
  (`self.Tree_location`))