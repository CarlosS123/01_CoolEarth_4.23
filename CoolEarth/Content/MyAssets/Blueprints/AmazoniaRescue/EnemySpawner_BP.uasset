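; Spawner for the Amazonia Rescue game that periodically turns a random player plane into an enemy plane.
; A DoOnce on Tick waits a short random delay, destroys a random PLANES_Ch_Player_BP and spawns a PLANES_Ch_Enemy_BP at its transform.
; Each spawn resets the DoOnce to repeat the cycle until LevelComplete sets LevelFinished, which blocks further swaps.
; BeginPlay also shows the mouse cursor.
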(event `self.ReceiveBeginPlay`
  (set `PlayerController.bShowMouseCursor` true (`GameplayStatics.GetPlayerController` 0)))

(event `self.ReceiveTick`
  (params (DeltaSeconds :type "Float (single-precision)"))
  (`/Engine/EditorBlueprintResources/StandardMacros.DoOnce` false :!label _label
    (:`Completed`
      (`KismetSystemLibrary.Delay` (`KismetMathLibrary.RandomFloatInRange` 0.0 3.0))
      (bind _outactors (`GameplayStatics.GetAllActorsOfClass` "/Game/MyAssets/Blueprints/AmazoniaRescue/PLANES_Ch_Player_BP.PLANES_Ch_Player_BP_C"))
      (set `self.SelectedPlane` (`|GetArrayItem` _outactors (`KismetMathLibrary.RandomIntegerInRange` 0 (- (`KismetArrayLibrary.Array_Length` _outactors) 1))))
      (set `self.NewPlane` (`self.GetTransform` (`self.SelectedPlane`)))
      (if (not (`self.LevelFinished`))
        (`self.K2_DestroyActor` (`self.SelectedPlane`))
        (bind _returnvalue (`|SpawnActorFromClass` "/Game/MyAssets/Blueprints/AmazoniaRescue/PLANES_Ch_Enemy_BP.PLANES_Ch_Enemy_BP_C" (`self.NewPlane`) "Undefined" "OverrideRootScale" null false null))
        (`KismetSystemLibrary.PrintString` (`KismetSystemLibrary.GetDisplayName` _returnvalue))
        (`self.RestartSpawnCountDown`)))))

(event `RestartSpawnCountDown`
  (goto _label :!via `Reset`))

(event `LevelComplete`
  (params (complete :type Boolean))
  (set `self.LevelFinished` complete))

(fn `UserConstructionScript`)