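; CityGameHUD_BP is the city level's HUD Blueprint, which delegates menu and minigame instruction display to the CoolEarth_GI_Menu game instance.
; On BeginPlay it sends the current level name to the game instance as the city level, then shows the main menu widget and the default instructions.
; The HUD_ShowMiniGameInstructions event enables instructions on the game instance and shows those for the given minigame.
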(event `self.ReceiveBeginPlay`
  (`self.SendCityLevelNameToGameInstance`)
  (bind _ascool_earth_gi_menu (cast `/Game/MyAssets/Blueprints/CoolEarth_GI_Menu` (`GameplayStatics.GetGameInstance`)))
  (set `self.GameInstance_REF` _ascool_earth_gi_menu)
  (`/Game/MyAssets/Blueprints/CoolEarth_GI_Menu.Show MainMenu WB` (`self.GameInstance_REF`))
  ;[1 1 1] This is for displaying by default the last minigame instructions
  (`/Game/MyAssets/Blueprints/CoolEarth_GI_Menu.Show MainInstructions` (`self.GameInstance_REF`) "None"))

(event `HUD_ShowMiniGameInstructions`
  (params (MiniGameToDisplay :type Name))
  (`/Game/MyAssets/Blueprints/CoolEarth_GI_Menu.Set Can Show Instructions` (`self.GameInstance_REF`) true)
  (`/Game/MyAssets/Blueprints/CoolEarth_GI_Menu.Show MainInstructions` (`self.GameInstance_REF`) MiniGameToDisplay))

(fn `SendCityLevelNameToGameInstance`
  (bind _ascool_earth_gi_menu (cast `/Game/MyAssets/Blueprints/CoolEarth_GI_Menu` (`GameplayStatics.GetGameInstance`)))
  (bind _returnvalue (`GameplayStatics.GetCurrentLevelName` true))
  (`/Game/MyAssets/Blueprints/CoolEarth_GI_Menu.SetCityLevelName` _ascool_earth_gi_menu (`KismetStringLibrary.Conv_StringToName` _returnvalue)))

(fn `UserConstructionScript`)