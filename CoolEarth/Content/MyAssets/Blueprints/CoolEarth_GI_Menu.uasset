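; Game instance for CoolEarth menus that keeps level and minigame state and handles level travel.
; It lazily creates, caches and shows the main menu and minigame instruction widgets.
; Instructions appear only when a flag allows it, reusing the last selected minigame if no name is passed.
; It records the current level before travel and returns to the stored city level, falling back to the city selector.
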(event `Show MainMenu WB`
  (`/Engine/EditorBlueprintResources/StandardMacros.IsValid` (`self.MainMenu_Widget_REF`)
    (:`Is Valid`
      _)
    (:`Is Not Valid`
      (bind _returnvalue (`|CreateWidget` "/Game/MyAssets/Blueprints/UserInterface/MainMenu_WB.MainMenu_WB_C" (`GameplayStatics.GetPlayerController` 0)))
      (set `self.MainMenu_Widget_REF` _returnvalue)))
  (`UserWidget.AddToViewport` (`self.MainMenu_Widget_REF`) 0))

(event `SetCityLevelName`
  (params (`Level Name` :type Name))
  (set `self.CityLevel` `Level Name`))

(event `Set Can Show Instructions`
  (params (`Should Show Instructions` :type Boolean))
  ;[1 1 1] This is neccesary for specifying in the minigame if instructions should be displayed in the city level after the player leaves the minigame
  (set `self.CanShowInstructions` `Should Show Instructions`))

(event `Show MainInstructions`
  (params (MiniGameName :type Name))
  (bind _maininstructions_hud_ref (`self.MainInstructions_HUD_REF`))
  ;[1 1 1] This is neccesary for specifying in the minigame if instructions should be displayed in the city level after the player leaves the minigame
  (if (`self.CanShowInstructions`)
    (if (!= MiniGameName "None")
      (set `self.LastMiniGameSelected` MiniGameName))
    (`/Engine/EditorBlueprintResources/StandardMacros.IsValid` (`self.MainInstructions_HUD_REF`)
      (:`Is Valid`
        _)
      (:`Is Not Valid`
        (bind _returnvalue (`|CreateWidget` "/Game/MyAssets/Blueprints/UserInterface/MainInstructions_WB.MainInstructions_WB_C" (`GameplayStatics.GetPlayerController` 0)))
        (set `self.MainInstructions_HUD_REF` _returnvalue)))
    (`UserWidget.AddToViewport` _maininstructions_hud_ref 0)
    (`/Game/MyAssets/Blueprints/UserInterface/MainInstructions_WB.SetMinigame` _maininstructions_hud_ref (`self.LastMiniGameSelected`))))

(event `OpenLevel`
  (params (LevelToOpen :type Name))
  (bind _returnvalue (`GameplayStatics.GetCurrentLevelName` true))
  (set `self.LastLevelOpened` (`KismetStringLibrary.Conv_StringToName` _returnvalue))
  (`GameplayStatics.OpenLevel` LevelToOpen))

(event `OpenCityLevel`
  (if (!= (`self.CityLevel`) "None")
    (`GameplayStatics.OpenLevel` (`self.CityLevel`))
    (else
      (`GameplayStatics.OpenLevel` "CitySelector_LVL")
      (`KismetSystemLibrary.PrintString` "Level with default name" true true (struct :`G` 0.66 :`B` 1.0 :`A` 1.0) 5.0))))