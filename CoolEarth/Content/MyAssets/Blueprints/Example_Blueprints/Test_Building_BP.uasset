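; Test building Blueprint that procedurally lays out a square grid of random building meshes from its construction script.
; Nested loops up to Extend add static mesh components spaced by BuildingDistance on X and Y, each assigned a random mesh from Buildings.
; The outer loop also places a mesh per X step, overlapping the grid's first row at Y zero.
; The event graph has no active logic.
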(fn `UserConstructionScript`
  (bind _buildings (`self.Buildings`))
  (bind _buildingdistance (`self.BuildingDistance`))
  (bind _extend (`self.Extend`))
  (bind _output (`|GetArrayItem` _buildings (`KismetMathLibrary.RandomInteger` (`KismetArrayLibrary.Array_Length` _buildings))))
  (for _index (range (+ _extend 1))
    (bind _returnvalue (* _index _buildingdistance))
    (bind _returnvalue_2 (`AddComponent|NODE_AddStaticMeshComponent-0` :`RelativeTransform` (`KismetMathLibrary.MakeTransform` (`KismetMathLibrary.MakeVector` _returnvalue))))
    (`StaticMeshComponent.SetStaticMesh` _returnvalue_2 _output)
    (for _index_2 (range (+ _extend 1))
      (bind _returnvalue_3 (`AddComponent|NODE_AddStaticMeshComponent-1` :`RelativeTransform` (`KismetMathLibrary.MakeTransform` (`KismetMathLibrary.MakeVector` _returnvalue (* _index_2 _buildingdistance)))))
      (`StaticMeshComponent.SetStaticMesh` _returnvalue_3 _output))))