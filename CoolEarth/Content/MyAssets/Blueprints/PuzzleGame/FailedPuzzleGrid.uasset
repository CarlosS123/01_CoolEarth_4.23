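; Puzzle grid actor, named as a failed attempt, that turns a static mesh into a sliding-apart 3x3 set of procedural mesh pieces on BeginPlay.
; It copies the mesh, cuts it along X and Y with SliceProceduralMesh, stores the halves in Grid and offsets outer pieces to form gaps.
; GridRandomization records and shuffles piece locations but never applies them, instead moving every piece to world origin.
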(event `self.ReceiveBeginPlay`
  (bind _output (`|GetArrayItem` (`self.Grid`) 2))
  (bind _output_2 (`|GetArrayItem` (`self.Grid`)))
  (`KismetProceduralMeshLibrary.CopyProceduralMeshFromStaticMeshComponent` (`self.MeshToCopy`) 0 (`self.ProceduralMesh`))
  (switch `int` 0
    (:`0`
      (`KismetArrayLibrary.Array_Add` (`self.Grid`) (`self.ProceduralMesh`))
      (bind _outotherhalfprocmesh (`KismetProceduralMeshLibrary.SliceProceduralMesh` (`|GetArrayItem` (`self.Grid`)) (366.0 0.0 0.0) (1.0 0.0 0.0) true "NoCap"))
      (`KismetArrayLibrary.Array_Add` (`self.Grid`) _outotherhalfprocmesh)
      (bind _outotherhalfprocmesh_2 (`KismetProceduralMeshLibrary.SliceProceduralMesh` _outotherhalfprocmesh (-333.0 0.0 0.0) (1.0 0.0 0.0) true "NoCap"))
      (`KismetArrayLibrary.Array_Add` (`self.Grid`) _outotherhalfprocmesh_2)
      (`SceneComponent.K2_SetWorldLocation` _output_2 (+ (`SceneComponent.K2_GetComponentLocation` _output_2) (100.0 0.0 0.0)) false false)
      (`SceneComponent.K2_SetWorldLocation` _output (- (`SceneComponent.K2_GetComponentLocation` _output) (100.0 0.0 0.0)) false false)
      (for _index (range 3)
        (bind _outotherhalfprocmesh_3 (`KismetProceduralMeshLibrary.SliceProceduralMesh` (`|GetArrayItem` (`self.Grid`) _index) (0.0 -333.0 0.0) (0.0 1.0 0.0) true "NoCap"))
        (bind _returnvalue (`KismetArrayLibrary.Array_Add` (`self.Grid`) _outotherhalfprocmesh_3))
        (bind _outotherhalfprocmesh_4 (`KismetProceduralMeshLibrary.SliceProceduralMesh` (`|GetArrayItem` (`self.Grid`) _index) (0.0 333.0 0.0) (0.0 1.0 0.0) true "NoCap"))
        (`KismetArrayLibrary.Array_Add` (`self.Grid`) _outotherhalfprocmesh_4)
        (bind _output_3 (`|GetArrayItem` (`self.Grid`) _index))
        (`SceneComponent.K2_SetWorldLocation` _output_3 (+ (`SceneComponent.K2_GetComponentLocation` _output_3) (0.0 100.0 0.0)) false false)
        (bind _output_4 (`|GetArrayItem` (`self.Grid`) _returnvalue))
        (`SceneComponent.K2_SetWorldLocation` _output_4 (- (`SceneComponent.K2_GetComponentLocation` _output_4) (0.0 100.0 0.0)) false false))
      (`self.GridRandomization`))))

(event `GridRandomization`
  (for _array_element (`self.Grid`)
    (bind _returnvalue (`SceneComponent.K2_GetComponentLocation` _array_element))
    (`KismetArrayLibrary.Array_Add` (`self.GridLocations`) _returnvalue)
    (`KismetArrayLibrary.Array_Add` (`self.RandomizedGridLocations`) _returnvalue))
  (`KismetArrayLibrary.Array_Shuffle` (`self.RandomizedGridLocations`))
  (for (_array_element_2 _array_index) (`self.Grid`)
    (`SceneComponent.K2_SetWorldLocation` _array_element_2 (0.0 0.0 0.0) false false)))

(fn `UserConstructionScript`)