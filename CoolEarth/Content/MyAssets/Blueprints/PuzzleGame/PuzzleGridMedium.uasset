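; Medium sliding-tile puzzle actor with twelve square meshes, played by touch.
; BeginPlay records solved positions, shuffles the tiles across them and hides one of the first nine as the empty slot.
; A touched tile swaps with that slot when 120 units away along X or Y, then all positions are compared to the solved layout.
; PuzzleHUD_BP receives every click count and GameOver on completion, with the hidden tile's index passed as TimeLeft.
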(event `self.ReceiveBeginPlay`
  (bind _tiles (`self.Tiles`))
  (set `self.TileToDisappear` (`KismetMathLibrary.RandomIntegerInRange` 0 8))
  (`KismetArrayLibrary.Array_Add` _tiles (`self.Square1`))
  (`KismetArrayLibrary.Array_Add` _tiles (`self.Square2`))
  (`KismetArrayLibrary.Array_Add` _tiles (`self.Square3`))
  (`KismetArrayLibrary.Array_Add` _tiles (`self.Square4`))
  (`KismetArrayLibrary.Array_Add` _tiles (`self.Square5`))
  (`KismetArrayLibrary.Array_Add` _tiles (`self.Square6`))
  (`KismetArrayLibrary.Array_Add` _tiles (`self.Square7`))
  (`KismetArrayLibrary.Array_Add` _tiles (`self.Square8`))
  (`KismetArrayLibrary.Array_Add` _tiles (`self.Square9`))
  (`KismetArrayLibrary.Array_Add` _tiles (`self.Square10`))
  (`KismetArrayLibrary.Array_Add` _tiles (`self.Square11`))
  (`KismetArrayLibrary.Array_Add` _tiles (`self.Square12`))
  (for _array_element (`self.Tiles`)
    (bind _returnvalue (`SceneComponent.K2_GetComponentLocation` _array_element))
    (`KismetArrayLibrary.Array_Add` (`self.Locations`) _returnvalue)
    (`KismetArrayLibrary.Array_Add` (`self.RandomizedLocations`) _returnvalue))
  (`KismetArrayLibrary.Array_Shuffle` (`self.RandomizedLocations`))
  (for (_array_element_2 _array_index) (`self.Tiles`)
    (`SceneComponent.K2_SetWorldLocation` _array_element_2 (`|GetArrayItem` (`self.RandomizedLocations`) _array_index) false false))
  (`SceneComponent.SetVisibility` (`|GetArrayItem` (`self.Tiles`) (`self.TileToDisappear`)) false false)
  (set `PlayerController.bShowMouseCursor` true (`GameplayStatics.GetPlayerController` 0)))

(event `self.Square1.OnInputTouchEnd`
  (params (FingerIndex :type "ETouchIndex Enum" :default "Touch1") (TouchedComponent :type "PrimitiveComponent Object Reference"))
  (`self.Clicked` TouchedComponent))

(event `Clicked`
  (params (ClickedMesh :type "PrimitiveComponent Object Reference"))
  (bind _returnvalue (`SceneComponent.K2_GetComponentLocation` ClickedMesh))
  (bind _iscomplete (`self.IsComplete`))
  (bind _iscomplete_2 (`self.IsComplete`))
  (bind _output (`|GetArrayItem` (`self.Tiles`) (`self.TileToDisappear`)))
  (bind _returnvalue_2 (`SceneComponent.K2_GetComponentLocation` (`|GetArrayItem` (`self.Tiles`) (`self.TileToDisappear`))))
  (bind _output_get (set `self.Clicks` (+ (`self.Clicks`) 1)))
  (bind _aspuzzle_hud_bp (cast `/Game/MyAssets/Blueprints/PuzzleGame/PuzzleHUD_BP` (`PlayerController.GetHUD` (`GameplayStatics.GetPlayerController` 0))))
  (`/Game/MyAssets/Blueprints/PuzzleGame/PuzzleHUD_BP.Clicked` _aspuzzle_hud_bp _output_get)
  (if (or (== (+ _returnvalue (0.0 120.0 0.0)) _returnvalue_2 :`ErrorTolerance` 1.0) (== (+ _returnvalue (0.0 -120.0 0.0)) _returnvalue_2 :`ErrorTolerance` 1.0) (== (+ _returnvalue (120.0 0.0 0.0)) _returnvalue_2 :`ErrorTolerance` 1.0) (== (+ _returnvalue (-120.0 0.0 0.0)) _returnvalue_2 :`ErrorTolerance` 1.0))
    (set `self.OldEmptyLocation` (`SceneComponent.K2_GetComponentLocation` _output))
    (`SceneComponent.K2_SetWorldLocation` _output _returnvalue false false)
    (`SceneComponent.K2_SetWorldLocation` ClickedMesh (`self.OldEmptyLocation`) false false)
    (for (_array_element _array_index) (`self.Tiles`)
      (if (== (`|GetArrayItem` (`self.Locations`) _array_index) (`SceneComponent.K2_GetComponentLocation` _array_element) :`ErrorTolerance` 1.0)
        (`KismetArrayLibrary.Array_Set` _iscomplete _array_index true)
        (else
          (`KismetArrayLibrary.Array_Set` _iscomplete _array_index))))
    (if (and (`|GetArrayItem` _iscomplete_2) (`|GetArrayItem` _iscomplete_2 1) (`|GetArrayItem` _iscomplete_2 2) (`|GetArrayItem` _iscomplete_2 3) (`|GetArrayItem` _iscomplete_2 4) (`|GetArrayItem` _iscomplete_2 5) (`|GetArrayItem` _iscomplete_2 6) (`|GetArrayItem` _iscomplete_2 7) (`|GetArrayItem` _iscomplete_2 8) (`|GetArrayItem` _iscomplete_2 9) (`|GetArrayItem` _iscomplete_2 10) (`|GetArrayItem` _iscomplete_2 11))
      (bind _aspuzzle_hud_bp_2 (cast `/Game/MyAssets/Blueprints/PuzzleGame/PuzzleHUD_BP` (`PlayerController.GetHUD` (`GameplayStatics.GetPlayerController` 0))))
      (`/Game/MyAssets/Blueprints/PuzzleGame/PuzzleHUD_BP.GameOver` _aspuzzle_hud_bp_2 (`self.Clicks`) (`self.TileToDisappear`)))))

(event `self.Square2.OnInputTouchEnd`
  (params (FingerIndex :type "ETouchIndex Enum" :default "Touch1") (TouchedComponent :type "PrimitiveComponent Object Reference"))
  (`self.Clicked` TouchedComponent))

(event `self.Square3.OnInputTouchEnd`
  (params (FingerIndex :type "ETouchIndex Enum" :default "Touch1") (TouchedComponent :type "PrimitiveComponent Object Reference"))
  (`self.Clicked` TouchedComponent))

(event `self.Square4.OnInputTouchEnd`
  (params (FingerIndex :type "ETouchIndex Enum" :default "Touch1") (TouchedComponent :type "PrimitiveComponent Object Reference"))
  (`self.Clicked` TouchedComponent))

(event `self.Square5.OnInputTouchEnd`
  (params (FingerIndex :type "ETouchIndex Enum" :default "Touch1") (TouchedComponent :type "PrimitiveComponent Object Reference"))
  (`self.Clicked` TouchedComponent))

(event `self.Square6.OnInputTouchEnd`
  (params (FingerIndex :type "ETouchIndex Enum" :default "Touch1") (TouchedComponent :type "PrimitiveComponent Object Reference"))
  (`self.Clicked` TouchedComponent))

(event `self.Square7.OnInputTouchEnd`
  (params (FingerIndex :type "ETouchIndex Enum" :default "Touch1") (TouchedComponent :type "PrimitiveComponent Object Reference"))
  (`self.Clicked` TouchedComponent))

(event `self.Square8.OnInputTouchEnd`
  (params (FingerIndex :type "ETouchIndex Enum" :default "Touch1") (TouchedComponent :type "PrimitiveComponent Object Reference"))
  (`self.Clicked` TouchedComponent))

(event `self.Square9.OnInputTouchEnd`
  (params (FingerIndex :type "ETouchIndex Enum" :default "Touch1") (TouchedComponent :type "PrimitiveComponent Object Reference"))
  (`self.Clicked` TouchedComponent))

(event `self.Square10.OnInputTouchEnd`
  (params (FingerIndex :type "ETouchIndex Enum" :default "Touch1") (TouchedComponent :type "PrimitiveComponent Object Reference"))
  (`self.Clicked` TouchedComponent))

(event `self.Square11.OnInputTouchEnd`
  (params (FingerIndex :type "ETouchIndex Enum" :default "Touch1") (TouchedComponent :type "PrimitiveComponent Object Reference"))
  (`self.Clicked` TouchedComponent))

(event `self.Square12.OnInputTouchEnd`
  (params (FingerIndex :type "ETouchIndex Enum" :default "Touch1") (TouchedComponent :type "PrimitiveComponent Object Reference"))
  (`self.Clicked` TouchedComponent))

(fn `UserConstructionScript`)