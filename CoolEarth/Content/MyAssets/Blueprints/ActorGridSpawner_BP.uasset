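; Actor spawner that fills a box from its location toward BoundCorner with randomly chosen ActorsToSpawn classes at BeginPlay.
; GridSpawn steps nested X, Y and Z loops by DistanceBetweenActors along world axes, using Density as a percentage chance per cell.
; Spawns get random location, rotation and uniform scale offsets.
; Z stacking is nested inside the Y loop, so the first Y row stays single-layer; the Spawns array loop does nothing.
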(event `self.ReceiveBeginPlay`
  (`self.GridSpawn`)
  (for _ (`self.Spawns`)
    _))

(fn `GridSpawn`
  (bind (_returnvalue_x _returnvalue_y _returnvalue_z) (`KismetMathLibrary.BreakVector` (`self.K2_GetActorLocation`)))
  (bind _actorstospawn (`self.ActorsToSpawn`))
  (bind _locationrandomness (`self.LocationRandomness`))
  (bind _rotationrandomness (`self.RotationRandomness`))
  (bind _classtospawn (`self.classToSpawn`))
  (bind _scalerandomness (`self.ScaleRandomness`))
  (bind (_boundcorner_x _boundcorner_y _boundcorner_z) (`KismetMathLibrary.BreakVector` (`self.BoundCorner`)))
  (bind _distancebetweenactors (`self.DistanceBetweenActors`))
  (bind (_out_x _out_y _out_z) (`KismetMathLibrary.BreakVector` (`/Game/MyAssets/Blueprints/myVectorFunctions_BL.RandomVectorInRange` (`KismetMathLibrary.NegateVector` _locationrandomness) _locationrandomness)))
  (bind _out (`/Game/MyAssets/Blueprints/myVectorFunctions_BL.RandomRotatorInRange` (`KismetMathLibrary.NegateRotator` _rotationrandomness) _rotationrandomness))
  (bind _returnvalue (>= (`self.Density`) (* (`KismetMathLibrary.RandomFloat`) 100.0)))
  (bind _returnvalue_2 (- (`KismetMathLibrary.FTrunc` (/ _boundcorner_y _distancebetweenactors)) 0))
  (bind _returnvalue_3 (`KismetMathLibrary.RandomFloatInRange` (+ (* _scalerandomness -1.0) 1.0) (+ _scalerandomness 1.0)))
  (bind _returnvalue_4 (- (`KismetMathLibrary.FTrunc` (/ _boundcorner_z (`self.DistanceBetweenActors`))) 0))
  (bind _output (`|GetArrayItem` _actorstospawn (`KismetMathLibrary.RandomInteger` (`KismetArrayLibrary.Array_Length` _actorstospawn))))
  (for _index (range (+ (- (`KismetMathLibrary.FTrunc` (/ _boundcorner_x _distancebetweenactors)) 0) 1))
    (bind _output_get (set `self.classToSpawn` _output))
    (if (`KismetSystemLibrary.IsValidClass` _output_get)
      (if _returnvalue
        (bind _returnvalue_5 (+ _returnvalue_x (* _index (`self.DistanceBetweenActors`))))
        (`|SpawnActorFromClass` _classtospawn (`KismetMathLibrary.MakeTransform` (`KismetMathLibrary.MakeVector` (+ _returnvalue_5 _out_x) (+ _returnvalue_y _out_y) (+ _returnvalue_z _out_z)) _out (`KismetMathLibrary.Conv_DoubleToVector` _returnvalue_3)) "Undefined" "OverrideRootScale" self null)))
    (if (>= _returnvalue_2 1)
      (for _index_2 (range 1 (+ _returnvalue_2 1))
        (bind _output_get_2 (set `self.classToSpawn` _output))
        (if (`KismetSystemLibrary.IsValidClass` _output_get_2)
          (if _returnvalue
            (bind _returnvalue_6 (+ _returnvalue_y (* _index_2 (`self.DistanceBetweenActors`))))
            (`|SpawnActorFromClass` _classtospawn (`KismetMathLibrary.MakeTransform` (`KismetMathLibrary.MakeVector` (+ _returnvalue_5 _out_x) (+ _returnvalue_6 _out_y) (+ _returnvalue_z _out_z)) _out (`KismetMathLibrary.Conv_DoubleToVector` _returnvalue_3)) "Undefined" "OverrideRootScale" self null)))
        (if (>= _returnvalue_4 1)
          (for _index_3 (range 1 (+ _returnvalue_4 1))
            (bind _output_get_3 (set `self.classToSpawn` _output))
            (if (`KismetSystemLibrary.IsValidClass` _output_get_3)
              (if _returnvalue
                (`|SpawnActorFromClass` _classtospawn (`KismetMathLibrary.MakeTransform` (`KismetMathLibrary.MakeVector` (+ _out_x _returnvalue_5) (+ _out_y _returnvalue_6) (+ _out_z (+ _returnvalue_z (* _index_3 (`self.DistanceBetweenActors`))))) _out (`KismetMathLibrary.Conv_DoubleToVector` _returnvalue_3)) "Undefined" "OverrideRootScale" self null)))))))))

(fn `UserConstructionScript`)