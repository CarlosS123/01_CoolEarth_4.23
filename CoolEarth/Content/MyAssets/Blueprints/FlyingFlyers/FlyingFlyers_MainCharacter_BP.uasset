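; Flying Flyers main character Blueprint that snaps its mesh to one of four fixed world yaw directions from touch swipes or movement axis input.
; Touch movement past SwipeTreshold on X or Y fires a per-direction DoOnce, re-armed on release, while MoveForward and MoveRight drive the same rotations directly.
; BeginPlay shows the mouse cursor; movement, snake spline and camera nodes are unconnected leftovers.
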(event `Key|A`
  (params (Key :type "Key Structure")))

(event `Key|S`
  (params (Key :type "Key Structure")))

(event `InputTouch`
  (params (Location :type "Vector Structure") (FingerIndex :type "ETouchIndex Enum"))
  (bind _returnvalue (`|EnumEquality` FingerIndex "Touch1"))
  (bind _mesh (`self.Mesh`))
  (bind (_initialfinger_x _initialfinger_y) (`KismetMathLibrary.BreakVector` (`self.InitialFinger`)))
  (bind _swipetreshold (`self.SwipeTreshold`))
  (bind _returnvalue_2 (- (.y Location) _initialfinger_y))
  (bind _returnvalue_3 (- (.x Location) _initialfinger_x))
  (bind _returnvalue_4 (* _swipetreshold -1.0))
  (:`Pressed`
    (if _returnvalue
      (set `self.InitialFinger` Location)
      (`KismetSystemLibrary.PrintString` "Touch")))
  (:`Released`
    (set `self.InitialFinger` (0.0 0.0 0.0))
    (`|ExecutionSequence`
      (:`then_0`
        (goto _label :!via `Reset`))
      (:`then_1`
        (goto _label_3 :!via `Reset`))
      (:`then_2`
        (goto _label_5 :!via `Reset`))
      (:`then_3`
        (goto _label_7 :!via `Reset`))))
  (:`Moved`
    (if _returnvalue
      (`|ExecutionSequence`
        (:`then_0`
          (`KismetSystemLibrary.PrintString` (`KismetStringLibrary.Conv_DoubleToString` _returnvalue_3))
          (if (> _returnvalue_3 _swipetreshold)
            (`/Engine/EditorBlueprintResources/StandardMacros.DoOnce` false :!label _label
              (:`Completed`
                (`SceneComponent.K2_SetWorldRotation` :`self` _mesh :!label _label_2)))
            (elif (< _returnvalue_3 _returnvalue_4)
              (`/Engine/EditorBlueprintResources/StandardMacros.DoOnce` false :!label _label_3
                (:`Completed`
                  (`SceneComponent.K2_SetWorldRotation` _mesh (struct :`Yaw` 180.0) false false :!label _label_4))))))
        (:`then_1`
          (if (> _returnvalue_2 _swipetreshold)
            (`/Engine/EditorBlueprintResources/StandardMacros.DoOnce` false :!label _label_5
              (:`Completed`
                (`SceneComponent.K2_SetWorldRotation` _mesh (struct :`Yaw` 90.0) false false :!label _label_6)))
            (elif (< _returnvalue_2 _returnvalue_4)
              (`/Engine/EditorBlueprintResources/StandardMacros.DoOnce` false :!label _label_7
                (:`Completed`
                  (`SceneComponent.K2_SetWorldRotation` _mesh (struct :`Yaw` -90.0) false false :!label _label_8))))))))))

(event `InputAxis|MoveForward`
  (params (AxisValue :type "Float (single-precision)"))
  (if (> AxisValue 0.5)
    (goto _label_8)
    (elif (< AxisValue -0.5)
      (goto _label_6))))

(event `InputAxis|MoveRight`
  (params (AxisValue :type "Float (single-precision)"))
  (if (> AxisValue 0.5)
    (goto _label_2)
    (elif (< AxisValue -0.5)
      (goto _label_4))))

(event `self.ReceiveBeginPlay`
  (set `PlayerController.bShowMouseCursor` true (`GameplayStatics.GetPlayerController` 0)))

(fn `UserConstructionScript`)