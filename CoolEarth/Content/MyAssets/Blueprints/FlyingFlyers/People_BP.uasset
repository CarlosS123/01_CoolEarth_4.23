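; People_BP is a collectible person in Flying Flyers that joins the SnakeCharacter's trail of followers.
; On first capsule overlap with the snake, it adds a follower on the HUD, registers with the snake, then marks itself following after a short delay.
; Once following, touching the snake destroys it, and touching another following person destroys both.
; A game-over flag disables these overlap reactions.
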(event `self.CapsuleComponent.OnComponentBeginOverlap`
  (params (OverlappedComponent :type "PrimitiveComponent Object Reference") (OtherActor :type "Actor Object Reference") (OtherComp :type "PrimitiveComponent Object Reference") (OtherBodyIndex :type Integer) (bFromSweep :type Boolean) (SweepResult :type "HitResult Structure (by ref)"))
  (if (not (`self.is Game Over`))
    (if (`self.isFollowing`)
      (cast `SnakeCharacter` OtherActor
        (:`then`
          (`self.K2_DestroyActor`))
        (:`CastFailed`
          (bind _aspeople_bp (cast `/Game/MyAssets/Blueprints/FlyingFlyers/People_BP` OtherActor))
          (if (`/Game/MyAssets/Blueprints/FlyingFlyers/People_BP.isFollowing` _aspeople_bp)
            (`self.K2_DestroyActor` _aspeople_bp)
            (`self.K2_DestroyActor`))))
      (else
        (bind _assnake_character (cast `SnakeCharacter` OtherActor))
        (`/Engine/EditorBlueprintResources/StandardMacros.DoOnce` false
          (:`Completed`
            (bind _asflying_flyers_hud_bp (cast `/Game/MyAssets/Blueprints/FlyingFlyers/FlyingFlyersHUD_BP` (`PlayerController.GetHUD` (`GameplayStatics.GetPlayerController` 0))))
            (`/Game/MyAssets/Blueprints/FlyingFlyers/FlyingFlyersHUD_BP.AddFollower` _asflying_flyers_hud_bp)
            (`SnakeCharacter.following` _assnake_character self)
            (`KismetSystemLibrary.Delay` 0.2)
            (set `self.isFollowing` true)))))))

(event `Set Game Is Over`
  (set `self.is Game Over` true))

(event `GetKilled`)

(fn `UserConstructionScript`)