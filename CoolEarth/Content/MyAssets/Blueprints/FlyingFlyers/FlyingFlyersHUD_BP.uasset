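; HUD Blueprint for FlyingFlyers that runs the round countdown, tracks the follower score and triggers game over.
; BeginPlay reads the duration from the game mode and creates the HUD widget.
; Tick pushes remaining time, measured against game time, to the widget; at zero it flags the player character and all People_BP actors once, then calls ShowWin.
; AddFollower increments the count shown as the score.
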(event `self.ReceiveBeginPlay`
  (`parent.ReceiveBeginPlay`)
  (bind _asflying_flyers_gm (cast `/Game/MyAssets/Blueprints/FlyingFlyers/FlyingFlyers_GM` (`GameplayStatics.GetGameMode`)))
  (set `self.GameTimer` (`/Game/MyAssets/Blueprints/FlyingFlyers/FlyingFlyers_GM.GameTime` _asflying_flyers_gm))
  (`/Engine/EditorBlueprintResources/StandardMacros.IsValid` (`self.hudWidget_Ref`)
    (:`Is Valid`
      _)
    (:`Is Not Valid`
      (bind _returnvalue (`|CreateWidget` "/Game/MyAssets/Blueprints/FlyingFlyers/FlyingFlyersHUD_WB.FlyingFlyersHUD_WB_C" (`GameplayStatics.GetPlayerController` 0)))
      (set `self.hudWidget_Ref` _returnvalue)))
  (`UserWidget.AddToViewport` (`self.hudWidget_Ref`) 0))

(event `self.ReceiveTick`
  (params (DeltaSeconds :type "Float (single-precision)"))
  (bind _returnvalue (- (`self.GameTimer`) (`KismetSystemLibrary.GetGameTimeInSeconds`)))
  (`parent.ReceiveTick` DeltaSeconds)
  (if (> _returnvalue 0.0)
    (set `/Game/MyAssets/Blueprints/FlyingFlyers/FlyingFlyersHUD_WB.TimeRemaining` _returnvalue (`self.hudWidget_Ref`))
    (else
      (`/Engine/EditorBlueprintResources/StandardMacros.DoOnce` false
        (:`Completed`
          (set `/Game/MyAssets/Blueprints/FlyingFlyers/FlyingFlyersHUD_WB.TimeRemaining` 0.0 (`self.hudWidget_Ref`))
          (bind _asflying_flyers_main_character_bp (cast `/Game/MyAssets/Blueprints/FlyingFlyers/FlyingFlyers_MainCharacter_BP` (`Controller.K2_GetPawn` (`GameplayStatics.GetPlayerController` 0))))
          (`/Game/MyAssets/Blueprints/FlyingFlyers/FlyingFlyers_MainCharacter_BP.Set Game Over` _asflying_flyers_main_character_bp)
          (bind _outactors (`GameplayStatics.GetAllActorsOfClass` "/Game/MyAssets/Blueprints/FlyingFlyers/People_BP.People_BP_C"))
          (for _array_element _outactors
            (`/Game/MyAssets/Blueprints/FlyingFlyers/People_BP.Set Game Is Over` _array_element))
          (`self.ShowWin`))))))

(event `AddFollower`
  (`/Engine/EditorBlueprintResources/StandardMacros.IncrementInt` (`self.Followers`)
    (:`  `
      (set `/Game/MyAssets/Blueprints/FlyingFlyers/FlyingFlyersHUD_WB.ScoreCounter` (`self.Followers`) (`self.hudWidget_Ref`)))))

(fn `UserConstructionScript`
  (`parent.UserConstructionScript`))