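; PeopleSpawner_BP is the people spawner for the FlyingFlyers game, configured by the active game mode.
; On BeginPlay it casts the game mode to FlyingFlyers_GM and copies its Density before calling the parent BeginPlay.
; The graph holds no spawning logic of its own, and a failed cast skips the parent call.
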(event `self.ReceiveBeginPlay`
  (bind _asflying_flyers_gm (cast `/Game/MyAssets/Blueprints/FlyingFlyers/FlyingFlyers_GM` (`GameplayStatics.GetGameMode`)))
  (set `self.Density` (`/Game/MyAssets/Blueprints/FlyingFlyers/FlyingFlyers_GM.Density` _asflying_flyers_gm))
  (`parent.ReceiveBeginPlay`))

(fn `UserConstructionScript`
  (`parent.UserConstructionScript`))