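; CityCharacter is a touch-controlled camera character that pans and zooms the view.
; While the first touch is held, Tick moves the actor in X and Y by the scaled frame-to-frame finger delta, printing a debug "Flick".
; Pinching opens a gate that lets the pinch axis change the camera arm length within zoom limits, and suspends panning until released.
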(event `InputAxis|PinchGesture`
  (params (AxisValue :type "Float (single-precision)"))
  (bind _cameraarm (`self.CameraArm`))
  (`/Engine/EditorBlueprintResources/StandardMacros.Gate` true :!label _label
    (:`Exit`
      (set `SpringArmComponent.TargetArmLength` (`KismetMathLibrary.FClamp` (+ (* (- (`self.CurrentAxis`) AxisValue) (`self.ZoomSpeed`)) (`SpringArmComponent.TargetArmLength` _cameraarm)) (`self.ZoomMaxIn`) (`self.ZoomMaxOut`)) _cameraarm)
      (set `self.CurrentAxis` AxisValue))))

(event `Key|Gesture_Pinch`
  (params (Key :type "Key Structure"))
  (:`Pressed`
    (set `self.IsZooming` true)
    (goto _label :!via `Open`))
  (:`Released`
    (set `self.IsZooming` false)
    (set `self.CurrentAxis` 1.0)
    (goto _label :!via `Close`)))

(event `InputAction|TouchOne`
  (params (Key :type "Key Structure"))
  (bind (_locationx _locationy) (`PlayerController.GetInputTouchState` (`GameplayStatics.GetPlayerController` 0) "Touch1"))
  (:`Pressed`
    (set `self.PreviousTouchLocation` (`KismetMathLibrary.MakeVector2D` _locationx _locationy))
    (set `self.IsMoving` true))
  (:`Released`
    (set `self.IsMoving` false)))

(event `self.ReceiveTick`
  (params (DeltaSeconds :type "Float (single-precision)"))
  (bind (_returnvalue_x _returnvalue_y _returnvalue_z) (`KismetMathLibrary.BreakVector` (`self.K2_GetActorLocation`)))
  (bind (_locationx _locationy) (`PlayerController.GetInputTouchState` (`GameplayStatics.GetPlayerController` 0) "Touch1"))
  (bind (_x _y) (`KismetMathLibrary.BreakVector2D` (- (`self.NewTouchLocation`) (`self.PreviousTouchLocation`))))
  (if (`self.IsZooming`)
    _
    (elif (`self.IsMoving`)
      (`KismetSystemLibrary.PrintString` "Flick")
      (set `self.NewTouchLocation` (`KismetMathLibrary.MakeVector2D` _locationx _locationy))
      (`self.K2_SetActorLocation` (`KismetMathLibrary.MakeVector` (+ (* _y (`self.ScrollMultiplier`)) _returnvalue_x) (+ (* (* _x -1.0) (`self.ScrollMultiplier`)) _returnvalue_y) _returnvalue_z))
      (set `self.PreviousTouchLocation` (`self.NewTouchLocation`)))))

(fn `UserConstructionScript`)